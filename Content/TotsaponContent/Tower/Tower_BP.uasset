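; Tower actor that targets SheepRunnerBase actors and spawns Bullet2 projectiles, using sprite, damage and fire rate from a data table row.
; Targets come from capsule overlaps or a throttled capsule trace at fixed world coordinates that picks the nearest sheep.
; Tick fires while the target is valid, with a Delay-based reload, and otherwise searches again.
; The HUD upgrade combo event is bound, but its handler is an empty stub.
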(event OnComponentBeginOverlap(Capsule)
  (params (OverlappedComponent :type Primitive%20Component%20Object%20Reference) (OtherActor :type Actor%20Object%20Reference) (OtherComp :type Primitive%20Component%20Object%20Reference) (OtherBodyIndex :type Integer) (bFromSweep :type Boolean) (SweepResult :type Hit%20Result%20Structure%20%28by%20ref%29))
  (Utilities|IsValid (Variables|Default|GettowerTarget)
    (:Is%20Not%20Valid
      (bind _assheep_runner_base (Utilities|Casting|CastToSheepRunnerBase OtherActor))
      (Variables|Default|SettowerTarget _assheep_runner_base))))

(event Custom|towerInit
  (Rendering|Components|Sprite|SetSprite (Variables|Default|GetcastleLevel1) (.towerSprite (Utilities|Struct|BreakTowerData (Variables|Default|GettowerData)))))

(event Custom|shoot
  (bind _towerdata (Variables|Default|GettowerData))
  (bind (_name _damage _firerate) (Utilities|Struct|BreakTowerData _towerdata))
  (Game|SpawnActorfromClass "/Game/TotsaponContent/Tower/bullet2.bullet2_C" (Transformation|GetWorldTransform (Variables|Default|GetbulletSpawn)) "Undefined" 0 _damage 0)
  (Development|PrintString "sadadssad")
  (Variables|Default|Setreload true)
  (Utilities|FlowControl|Delay _firerate)
  (Variables|Default|Setreload false))

(event Custom|findTarget
  (Variables|Default|SetisFindingNewTarget true)
  (bind (_outhits _returnvalue) (Class|KismetSystemLibrary|CapsuleTraceMultiforObjects "0,0.000000,1660.000000" "0.000000,0.000000,1660.000000" 2e+03 4e+02 (Utilities|Array|MakeArray "ObjectTypeQuery3") false 0 "ForOneFrame" true "(R=0.119021,G=0.000000,B=1.000000,A=1.000000)"))
  (if _returnvalue
    (bind _newtarget (CallFunction|GetNearestSheep _outhits))
    (Utilities|IsValid _newtarget
      (:Is%20Valid
        (Variables|Default|SettowerTarget _newtarget))
      (:Is%20Not%20Valid
        _)))
  (Utilities|FlowControl|Delay 0.25)
  (Variables|Default|SetisFindingNewTarget false))

(event Custom|comboToUpgrade
  (params (combo :type Integer))
  (if (== combo 0)
    _))

(event EventBeginPlay
  ;[1 1 1] Set up tower
  (bind _returnvalue (Utilities|GetDataTableRow "/Game/TotsaponContent/Tower/towerDataTable.towerDataTable" "1")
    (:then
      (Variables|Default|SettowerData _returnvalue)
      (CallFunction|TowerInit)
      (EventDispatchers|BindEventtoCallUpgradeTower (Variables|Default|Gethud) (delegate Custom|comboToUpgrade)))))

(event Collision|EventActorBeginOverlap
  (params (OtherActor :type Actor%20Object%20Reference)))

(event EventTick
  (params (DeltaSeconds :type Float%20%28single-precision%29))
  (Utilities|IsValid (Variables|Default|GettowerTarget)
    (:Is%20Valid
      (if (not (Variables|Default|Getreload))
        (CallFunction|Shoot)))
    (:Is%20Not%20Valid
      (if (not (Variables|Default|GetisFindingNewTarget))
        (CallFunction|FindTarget)))))

(fn ConstructionScript)

(fn GetNearestSheep
  (params (hitResults :type Array%20of%20Hit%20Result%20Structures))
  (for _array_element hitResults
    (bind _assheep_runner_base (Utilities|Casting|CastToSheepRunnerBase (.HitActor (Collision|BreakHitResult _array_element))))
    (Development|PrintString (Utilities|GetDisplayName _assheep_runner_base))
    (Utilities|IsValid (LocalVariables|GettempTarget)
      (:Is%20Valid
        (if (< (Math|Vector|VectorLength (- (Transformation|GetActorLocation) (Transformation|GetActorLocation (.HitActor (Collision|BreakHitResult _array_element))))) (LocalVariables|GettempDistance))
          (LocalVariables|SettempTarget _assheep_runner_base)
          (LocalVariables|SettempDistance (Math|Vector|VectorLength (- (Transformation|GetActorLocation) (Transformation|GetActorLocation (.HitActor (Collision|BreakHitResult _array_element))))))))
      (:Is%20Not%20Valid
        (LocalVariables|SettempTarget _assheep_runner_base)
        (LocalVariables|SettempDistance (Math|Vector|VectorLength (- (Transformation|GetActorLocation) (Transformation|GetActorLocation (.HitActor (Collision|BreakHitResult _array_element)))))))))
  (return (LocalVariables|GettempTarget)))